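; Mushroom pickup that the player collects by walking into its collision.
; On overlap it calls GetMushroom on any BP_ThirdPersonCharacter, then, only for player 0, flags itself collected, destroys itself and plays a 2D sound.
; Before destruction it passes itself to CallShroomCollected on BP_GameStateBase, which relays the event to the Level Blueprint.
; A separate UpdateMushroom event switches the sphere to an emissive pink material.
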(event OnComponentBeginOverlap(Collision)
  (params (OverlappedComponent :type Primitive%20Component%20Object%20Reference) (OtherActor :type Actor%20Object%20Reference) (OtherComp :type Primitive%20Component%20Object%20Reference) (OtherBodyIndex :type Integer) (bFromSweep :type Boolean) (SweepResult :type Hit%20Result%20Structure%20%28by%20ref%29))
  (bind _asbp_third_person_character (Utilities|Casting|CastToBP_ThirdPersonCharacter OtherActor))
  (Default|GetMushroom _asbp_third_person_character)
  (if (== (Game|GetPlayerCharacter 0) OtherActor)
    (Utilities|FlowControl|Sequence
      (:then_0
        (Variables|Default|SetHasBeenCollected true)
        ;[1 1 1] This calls the binded event on the level blueprint by going through the game state
        (bind _asbp_game_state_base (Utilities|Casting|CastToBP_GameStateBase (Game|GetGameState)))
        (Default|CallShroomCollected _asbp_game_state_base self)
        (Actor|DestroyActor))
      (:then_1
        (Audio|PlaySound2D "/Game/Audio/UI___Menu/UI___Menu/Signals/Inventory/Inventory_Nasty_Things_B.Inventory_Nasty_Things_B" 1.0 1.0 0.0 0 0)))))

(event Custom|UpdateMushroom
  (Rendering|Material|SetMaterial (Variables|Default|GetSphere) 0 "/Game/Materials/MI_EmissivePink.MI_EmissivePink"))

(fn ConstructionScript)