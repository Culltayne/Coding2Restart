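; BP_Weapon is a weapon Blueprint that holds a weapon type, damage type and damage range, and displays them as text.
; The randomizevalues event adds a small random amount to the current minimum damage, derives the maximum as that minimum plus a random spread, then calls Settext.
; Settext writes both enum names and the min-max damage range to three text components.
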(event Custom|randomizevalues
  (bind _output_get (Variables|Default|SetMin%20Dmg (+ (Variables|Default|GetMin%20Dmg) (Math|Random|RandomInteger 2))))
  (Variables|Default|SetMax%20Dmg (+ _output_get (Math|Random|RandomInteger 9)))
  (CallFunction|Settext))

(event Custom|Settext
  (Rendering|Components|TextRender|SetText (Variables|Default|GetTextWeaponType) (Utilities|Text|ToText(String) (Utilities|String|EnumtoString (Variables|Default|GetWeapon%20Type))))
  (Rendering|Components|TextRender|SetText (Variables|Default|GetTextElementType) (Utilities|Text|ToText(String) (Utilities|String|EnumtoString (Variables|Default|GetDamage%20Type))))
  (Rendering|Components|TextRender|SetText (Variables|Default|GetTextDamage) (Utilities|Text|ToText(String) (Utilities|String|Append (Utilities|String|ToString(Integer) (Variables|Default|GetMin%20Dmg)) " - " (Utilities|String|ToString(Integer) (Variables|Default|GetMax%20Dmg))))))

(fn ConstructionScript)