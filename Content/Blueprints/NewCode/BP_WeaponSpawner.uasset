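; BP_WeaponSpawner is a trigger actor that spawns a randomized weapon when a BP_ThirdPersonCharacter overlaps its sphere.
; SpawnWeapon picks a random DT_Weapons row and spawns a BP_Weapon at the sphere's location.
; It copies the row's weapon type, elemental type and base damage (as minimum damage) onto the weapon, then calls its Randomizevalues.
; Nothing limits repeat spawns, and an older text-display path is left unconnected.
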(event OnComponentBeginOverlap(Sphere)
  (params (OverlappedComponent :type Primitive%20Component%20Object%20Reference) (OtherActor :type Actor%20Object%20Reference) (OtherComp :type Primitive%20Component%20Object%20Reference) (OtherBodyIndex :type Integer) (bFromSweep :type Boolean) (SweepResult :type Hit%20Result%20Structure%20%28by%20ref%29))
  (Utilities|Casting|CastToBP_ThirdPersonCharacter OtherActor)
  (CallFunction|SpawnWeapon))

(event Custom|Spawn%20Weapon
  (bind _outrownames (DataTable|GetDataTableRowNames "/Game/Blueprints/DataTables/DT_Weapons.DT_Weapons"))
  (bind _returnvalue (Utilities|GetDataTableRow "/Game/Blueprints/DataTables/DT_Weapons.DT_Weapons" (.OutItem (Utilities|Array|Random _outrownames)))
    (:then
      (bind _returnvalue_2 (Game|SpawnActorfromClass "/Game/Blueprints/NewCode/BP_Weapon.BP_Weapon_C" (Math|Transform|MakeTransform (Transformation|GetWorldLocation (Variables|Default|GetSphere)) "0, 0, 0" "1.000000,1.000000,1.000000") "Undefined" "MultiplyWithRoot" 0 0))
      (Variables|/Game/Blueprints/NewCode/BP_Weapon.BP_Weapon_C|SetWeapon%20Type _returnvalue_2 (.weapontype _returnvalue))
      (Variables|/Game/Blueprints/NewCode/BP_Weapon.BP_Weapon_C|SetDamage%20Type _returnvalue_2 (.elementaltype _returnvalue))
      (Variables|/Game/Blueprints/NewCode/BP_Weapon.BP_Weapon_C|SetMin%20Dmg _returnvalue_2 (.basedamage _returnvalue))
      (Default|Randomizevalues _returnvalue_2))))

(event EventBeginPlay)

(event Collision|EventActorBeginOverlap
  (params (OtherActor :type Actor%20Object%20Reference)))

(event EventTick
  (params (DeltaSeconds :type Float%20%28single-precision%29)))

(fn ConstructionScript)